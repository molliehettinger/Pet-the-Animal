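; Pettable animal Blueprint that tracks friendship with whoever pets it.
; Interact lazily creates or reactivates a hearts Niagara effect, flags petting if not yet friends, and returns the animal name, friend status and scaled points; Endinteract stops both.
; While petted, Tick adds points per frame and sets IsFriend when raw points reach the freshly recomputed percentage, overwriting the BeginPlay value rather than using a fixed target.
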(event EventBeginPlay
  (Variables|Default|SetFriendship_add 1)
  (Variables|Default|SetFriendship_percentage (* (Variables|Default|GetFriendship_lvl) 400)))

(event Collision|EventActorBeginOverlap
  (params (OtherActor :type Actor%20Object%20Reference)))

(event EventTick
  (params (DeltaSeconds :type Float%20%28single-precision%29))
  (if (not (Variables|Default|GetIs_friend))
    (if (Variables|Default|GetBeing_pet)
      (Variables|Default|SetFriendship_points (+ (Variables|Default|GetFriendship_add) (Variables|Default|GetFriendship_points)))
      (Variables|Default|SetFriendship_percentage (/ (/ (Variables|Default|GetFriendship_points) (Variables|Default|GetFriendship_lvl)) 4))
      ;[1 1 1] Is this creature your friend
      (if (>= (Variables|Default|GetFriendship_points) (Variables|Default|GetFriendship_percentage))
        (Variables|Default|SetIs_friend true)))))

(fn ConstructionScript)

(fn Endinteract
  (bind _hearts_particles (Variables|Default|Gethearts_particles))
  (Utilities|IsValid _hearts_particles
    (:Is%20Valid
      (Components|Activation|Deactivate _hearts_particles)
      (if (Variables|Default|GetIs_friend)
        (Variables|Default|SetBeing_pet false)
        (return false)
        (else
          (Variables|Default|SetBeing_pet false)
          (return false))))))

(fn Interact
  (bind _animal_name (Variables|Default|GetAnimal_name))
  (bind _friendship_points (Variables|Default|GetFriendship_points))
  (bind _friendship_lvl (Variables|Default|GetFriendship_lvl))
  (bind _returnvalue (/ _friendship_points _friendship_lvl))
  (bind _returnvalue_2 (/ _returnvalue 4))
  (Utilities|IsValid (Variables|Default|Gethearts_particles)
    (:Is%20Valid
      (Components|Activation|Activate (Variables|Default|Gethearts_particles) false)
      (if (Variables|Default|GetIs_friend)
        (return true _returnvalue_2 _animal_name)
        (else
          (Variables|Default|SetBeing_pet true)
          (return false _returnvalue_2 _animal_name))))
    (:Is%20Not%20Valid
      (bind _returnvalue_3 (AddComponent|AddNiagaraComponent false (Math|Transform|MakeTransform (Transformation|GetActorLocation self) "0, 0, 0" "1.000000,1.000000,1.000000")))
      (Variables|Default|Sethearts_particles _returnvalue_3)
      (if (Variables|Default|GetIs_friend)
        (return true _returnvalue_2 _animal_name)
        (else
          (Variables|Default|SetBeing_pet true)
          (return false _returnvalue_2 _animal_name))))))