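; BP_PathActor is an AI helper actor that exposes a perch area and a spline path.
; On construction it stores its own location as the perch location and sizes its collision sphere to the Radius variable.
; Getters return the perch location with radius and the spline's length; the event graph has no active logic.
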(event EventBeginPlay)

(event Collision|EventActorBeginOverlap
  (params (OtherActor :type Actor%20Object%20Reference)))

(event EventTick
  (params (DeltaSeconds :type Float%20%28single-precision%29)))

(fn ConstructionScript
  (Variables|Default|SetPerchLocation (Transformation|GetActorLocation))
  (Components|Sphere|SetSphereRadius (Variables|Default|GetCollision) (Variables|Default|GetRadius) true))

(fn GetPerchInfo
  (return (Variables|Default|GetPerchLocation) (Variables|Default|GetRadius)))

(fn GetPathLength
  (return (Spline|GetSplineLength (Variables|Default|GetPath))))